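; BP_GraviFlipGameInstance is the GraviFlip game instance that handles online session teardown and connection errors.
; Network and travel error events print the failure type, then destroy the local player's session.
; A LeaveSession event opens MainMenuLevel and then destroys the session.
; A failed session destroy only prints a message.
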(event `self.HandleNetworkError`
  (params (FailureType :type "ENetworkFailure Enum" :default "NetDriverAlreadyExists") (bIsServer :type Boolean))
  ;[1 1 1] Handle Network & Travel Errors
  (`KismetSystemLibrary.PrintString` (`|GetEnumeratorNameAsString` FailureType) true true (struct :`R` 1.0 :`A` 1.0) 8.0)
  (`DestroySessionCallbackProxy.DestroySession` (`GameplayStatics.GetPlayerController` 0) :!label _label
    (:`OnFailure`
      (`KismetSystemLibrary.PrintString` "Failed To Destroy Session" true true (struct :`R` 1.0 :`A` 1.0) 5.0))))

(event `self.HandleTravelError`
  (params (FailureType :type "ETravelFailure Enum" :default "NoLevel"))
  ;[1 1 1] Handle Network & Travel Errors
  (`KismetSystemLibrary.PrintString` (`|GetEnumeratorNameAsString` FailureType) true true (struct :`R` 1.0 :`A` 1.0) 8.0)
  (goto _label))

(event `LeaveSession`
  ;[1 1 1] Leave Session
  (`GameplayStatics.OpenLevel` "MainMenuLevel")
  (`DestroySessionCallbackProxy.DestroySession` (`GameplayStatics.GetPlayerController` 0)
    (:`OnFailure`
      (`KismetSystemLibrary.PrintString` "Failed To Destroy Session" true true (struct :`R` 1.0 :`A` 1.0) 5.0))))