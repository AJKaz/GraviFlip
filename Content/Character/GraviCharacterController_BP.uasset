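; Player controller Blueprint for the Gravi character that handles the pause menu and input mode.
; On BeginPlay it sets game-only input, and the IA_Pause Enhanced Input action calls TogglePauseMenu.
; The toggle lazily creates and caches the WB_PauseMenu widget, then shows or collapses it, switching the mouse cursor and Game-and-UI or game-only input to match.
; The game itself is never paused.
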(event `self.ReceiveBeginPlay`
  (`WidgetBlueprintLibrary.SetInputMode_GameOnly` self))

(event `EnhancedInput|/Game/Character/Input/IA_Pause`
  (params (ActionValue :type Boolean) (ElapsedSeconds :type "Float (double-precision)") (TriggeredSeconds :type "Float (double-precision)") (InputAction :type "InputAction Object Reference" :default "/Game/Character/Input/IA_Pause.IA_Pause"))
  (:`Triggered`
    (`self.TogglePauseMenu`)))

(fn `TogglePauseMenu`
  (bind _wb_pausemenu (`self.WB_PauseMenu`))
  (`self.WB_PauseMenu`
    (:`then`
      (if (`Widget.IsVisible` (`self.WB_PauseMenu`))
        (`Widget.SetVisibility` _wb_pausemenu "Collapsed")
        (set `self.bShowMouseCursor` false)
        (`WidgetBlueprintLibrary.SetInputMode_GameOnly` self)
        (else
          (`Widget.SetVisibility` _wb_pausemenu "Visible")
          (set `self.bShowMouseCursor` true :!label _label)
          (`WidgetBlueprintLibrary.SetInputMode_GameAndUIEx` self (`self.WB_PauseMenu`)))))
    (:`else`
      (bind _returnvalue (`|CreateWidget` "/Game/Menus/Widgets/GameWidgets/WB_PauseMenu.WB_PauseMenu_C" self))
      (bind _output_get (set `self.WB_PauseMenu` _returnvalue))
      (`UserWidget.AddToViewport` _output_get 0)
      (goto _label))))

(fn `UserConstructionScript`)